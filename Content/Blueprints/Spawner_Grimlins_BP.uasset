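; Spawner actor that periodically spawns a configurable actor class, named for Gremlins, at its own transform.
; On BeginPlay it starts a looping timer at a configurable interval, and each tick of that timer calls Spawn and decrements a remaining-spawn counter.
; When the counter reaches zero, it clears and invalidates the timer, ending the spawning.
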(event Custom|Spawn_Gremlins
  (CallFunction|Spawn)
  (Variables|Default|SetMax_Spawn (- (Variables|Default|GetMax_Spawn) 1))
  (if (<= (Variables|Default|GetMax_Spawn) 0)
    (Utilities|Time|ClearandInvalidateTimerbyHandle (Variables|Default|GetTimer))))

(event EventBeginPlay
  (bind _returnvalue (Utilities|Time|SetTimerbyEvent (delegate Custom|Spawn_Gremlins) (Variables|Default|GetEvent%20Time) true))
  (Variables|Default|SetTimer _returnvalue))

(event Collision|EventActorBeginOverlap
  (params (OtherActor :type Actor%20Object%20Reference)))

(event EventTick
  (params (DeltaSeconds :type Float%20%28single-precision%29)))

(fn ConstructionScript)

(fn Spawn
  (Game|SpawnActorfromClass (Variables|Default|GetActor%20To%20Spawn) (Transformation|GetActorTransform) "Undefined" 0 0))