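; Light Blueprint that periodically switches its SpotLight on for a set duration, then off again.
; A looping timer started at BeginPlay fires Allume every EventLoop interval, which turns the light on only if it is hidden.
; Allume then starts a one-shot timer of ResteAlluméeTemps, whose CloseLight event toggles the light back and clears that timer handle.
; Both switches share LightOnOff, a visibility toggle rather than an explicit set.
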(event Custom|Allume
  (if (not (Variables|/Script/Engine.SceneComponent|GetbVisible (Variables|Default|GetSpotLight)))
    (CallFunction|LightOn/Off)
    (bind _returnvalue (Utilities|Time|SetTimerbyEvent (delegate Custom|Close%20light) (Variables|Default|GetReste%20Allumée%20%28temps%29)))
    (Variables|Default|SetTimer%20durée _returnvalue)))

(event Custom|Close%20light
  (CallFunction|LightOn/Off)
  (Utilities|Time|ClearandInvalidateTimerbyHandle (Variables|Default|GetTimer%20durée)))

(event EventBeginPlay
  (bind _returnvalue (Utilities|Time|SetTimerbyEvent (delegate Custom|Allume) (Variables|Default|GetEvent%20%28Loop%29%20) true))
  (Variables|Default|SetTimer%20loop _returnvalue))

(event Collision|EventActorBeginOverlap
  (params (OtherActor :type Actor%20Object%20Reference)))

(event EventTick
  (params (DeltaSeconds :type Float%20%28single-precision%29)))

(fn ConstructionScript)

(fn LightOn/Off
  (Rendering|ToggleVisibility (Variables|Default|GetSpotLight) false))