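; Spawner Blueprint that repeatedly spawns a configurable actor class a limited number of times.
; BeginPlay starts a looping timer that calls the Spawning event, which runs Spawn to create ActorToSpawn at the SpawnZone component's transform.
; Each call decrements MaxSpawn and clears the timer once it reaches zero or below.
; A DestroyActor call is left unconnected, so the spawner does not destroy itself.
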(event Custom|Spawning
  (CallFunction|Spawn)
  (Variables|Default|SetMax_Spawn (- (Variables|Default|GetMax_Spawn) 1))
  (if (<= (Variables|Default|GetMax_Spawn) 0)
    (Utilities|Time|ClearandInvalidateTimerbyHandle (Variables|Default|GetTimer))))

(event EventBeginPlay
  (bind _returnvalue (Utilities|Time|SetTimerbyEvent (delegate Custom|Spawning) (Variables|Default|GetEvent) true))
  (Variables|Default|SetTimer _returnvalue))

(event Collision|EventActorBeginOverlap
  (params (OtherActor :type Actor%20Object%20Reference)))

(fn ConstructionScript)

(fn Spawn
  (Game|SpawnActorfromClass (Variables|Default|GetActor%20to%20spawn) (Transformation|GetWorldTransform (Variables|Default|GetSpawn_Zone)) "Undefined" 0 0))