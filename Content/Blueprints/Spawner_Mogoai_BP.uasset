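; Spawner actor that emits Mogoai, or whatever class is set in ActorToSpawn, at its own transform.
; BeginPlay starts a looping timer on EventTime, and each tick of it calls SpawnMogoai and decrements MaxSpawn.
; The timer is cleared once MaxSpawn reaches zero, capping the total number spawned.
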(event Custom|Mogoai%20appear
  (CallFunction|SpawnMogoai)
  (Variables|Default|SetMax_Spawn (- (Variables|Default|GetMax_Spawn) 1))
  (if (<= (Variables|Default|GetMax_Spawn) 0)
    (Utilities|Time|ClearandInvalidateTimerbyHandle (Variables|Default|GetTimer))))

(event EventBeginPlay
  (bind _returnvalue (Utilities|Time|SetTimerbyEvent (delegate Custom|Mogoai%20appear) (Variables|Default|GetEvent%20Time) true))
  (Variables|Default|SetTimer _returnvalue))

(event Collision|EventActorBeginOverlap
  (params (OtherActor :type Actor%20Object%20Reference)))

(event EventTick
  (params (DeltaSeconds :type Float%20%28single-precision%29)))

(fn ConstructionScript)

(fn SpawnMogoai
  (Game|SpawnActorfromClass (Variables|Default|GetActorToSpawn) (Transformation|GetActorTransform) "Undefined" 0 0))