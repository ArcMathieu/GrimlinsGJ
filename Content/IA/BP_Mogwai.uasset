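; BP_Mogwai is an AI-driven Mogwai that walks to the first TargetPoint found in the level on BeginPlay.
; Kill freezes its movement, destroys it after a short delay and decrements the GremlinsGameMode Mogwai count.
; Duplicate spawns another BP_Mogwai at its transform and increments that count.
; GremlinTransformation replaces it with a BP_Gremlins at the same transform, leaving the count untouched.
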(event Custom|GremlinTransformation
  (Game|SpawnActorfromClass "/Game/IA/BP_Gremlins.BP_Gremlins_C" (Transformation|GetActorTransform) "Undefined" 0 0)
  (Actor|DestroyActor))

(event Custom|Kill
  (Pawn|Components|CharacterMovement|DisableMovement (Variables|Character|GetCharacterMovement))
  (Utilities|FlowControl|Delay 1.0)
  (Actor|DestroyActor)
  (bind _asgremlins_game_mode (Utilities|Casting|CastToGremlinsGameMode (Game|GetGameMode)))
  (Variables|/Game/GremlinsGameMode.GremlinsGameMode_C|SetCurrentMogwaiNb _asgremlins_game_mode (- (Variables|/Game/GremlinsGameMode.GremlinsGameMode_C|GetCurrentMogwaiNb _asgremlins_game_mode) 1)))

(event Custom|Duplicate
  (Game|SpawnActorfromClass "BP_Mogwai_C" (Transformation|GetActorTransform) "Undefined" 0 0)
  (bind _asgremlins_game_mode (Utilities|Casting|CastToGremlinsGameMode (Game|GetGameMode)))
  (Variables|/Game/GremlinsGameMode.GremlinsGameMode_C|SetCurrentMogwaiNb _asgremlins_game_mode (+ (Variables|/Game/GremlinsGameMode.GremlinsGameMode_C|GetCurrentMogwaiNb _asgremlins_game_mode) 1)))

(event EventBeginPlay
  (bind _outactors (Actor|GetAllActorsOfClass "/Script/Engine.TargetPoint"))
  (AI|AIMoveTo self "0, 0, 0" (Utilities|Array|Get(acopy) _outactors) 5.0 false))

(fn ConstructionScript)