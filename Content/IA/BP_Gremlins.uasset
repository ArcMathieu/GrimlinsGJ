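; Gremlin AI pawn that detects actors tagged Allies and reports them to its Blackboard as enemies.
; AI Perception updates set EnemyActor and InLineOfSight on a sensed ally and cancel the pending forget timer.
; Any other perception update starts a LineOfSightDuration timer that resets both keys.
; A self-repeating random wander via AIMoveTo is also defined, but its initial call is disconnected.
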(event OnTargetPerceptionUpdated(AIPerception)
  (params (Actor :type Actor%20Object%20Reference) (Stimulus :type AI%20Stimulus%20Structure))
  (bind _returnvalue (AI|GetBlackboard 0))
  ;[1 1 1] Cast value to BlackBoard
  (if (and (Actor|ActorHasTag Actor "Allies") (.bSuccessfullySensed (Utilities|Struct|BreakAIStimulus Stimulus)))
    (Utilities|Time|ClearandInvalidateTimerbyHandle (Variables|Default|GetLineOfSightTimer))
    (AI|Components|Blackboard|SetValueasBool _returnvalue (Variables|Default|GetIn%20Line%20Of%20Sight) true)
    (AI|Components|Blackboard|SetValueasObject _returnvalue (Variables|Default|GetEnemy%20Actor) Actor)
    (else
      (bind _returnvalue_2 (Utilities|Time|SetTimerbyEvent (delegate Custom|ResetBlackboard) (Variables|Default|GetLineOfSightDuration)))
      (Variables|Default|SetLineOfSightTimer _returnvalue_2))))

(event Custom|WalkToRdPos
  (bind _returnvalue (Transformation|GetActorLocation))
  (bind (_randomlocation _returnvalue_2) (AI|Navigation|GetRandomReachablePointinRadius _returnvalue 1e+03 0 0))
  (if _returnvalue_2
    (AI|AIMoveTo self _randomlocation 0 5.0 false
      (:OnSuccess
        (Utilities|FlowControl|Delay 3.0))
      (:OnFail
        (Utilities|FlowControl|Delay 0.2)))
    (CallFunction|WalktoRdPos)))

(event Custom|ResetBlackboard
  (bind _returnvalue (AI|GetBlackboard 0))
  ;[1 1 1] Cast value to BlackBoard
  (AI|Components|Blackboard|SetValueasBool _returnvalue (Variables|Default|GetIn%20Line%20Of%20Sight) false)
  (AI|Components|Blackboard|SetValueasObject _returnvalue (Variables|Default|GetEnemy%20Actor) 0))

(event EventBeginPlay)

(fn ConstructionScript)