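; GameMod_BP is a game-logic Blueprint that sets up a random choice between Light, Water and Food events.
; BeginPlay starts a one-shot 30-second timer for the light/water/food event, which rolls a random integer to branch with roughly equal odds into one of the three functions.
; The Light, Water and Food functions are empty stubs, so the choice has no effect yet.
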(event Custom|Light/water/food
  (Variables|Default|SetTemp_Int (Math|Random|RandomInteger 30))
  (if (> (Variables|Default|GetTemp_Int) 10)
    (if (> (Variables|Default|GetTemp_Int) 20)
      (CallFunction|Food)
      (else
        (CallFunction|Water)))
    (else
      (CallFunction|Light))))

(event EventBeginPlay
  (Utilities|Time|SetTimerbyEvent (delegate Custom|Light/water/food) 3e+01))

(event EventTick
  (params (DeltaSeconds :type Float%20%28single-precision%29)))

(fn ConstructionScript)

(fn Water)

(fn Light)

(fn Food)